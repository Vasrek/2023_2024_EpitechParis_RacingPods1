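; BP_Dummy is a placeholder pawn that shows the main menu and handles its gamepad and keyboard navigation.
; On BeginPlay it creates WBP_MainMenu, shows the cursor, sets Game and UI input mode, and highlights Play.
; D-pad or arrow keys step a clamped Index that calls the widget's hover functions for Play or Quit.
; Enter or the gamepad bottom face button calls the matching click function.
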(event EventBeginPlay
  (bind _returnvalue (Game|GetPlayerController 0))
  (bind _returnvalue_2 (UserInterface|CreateWidget "/Game/Blueprints/Widgets/WBP_MainMenu.WBP_MainMenu_C"))
  (bind _output_get (Variables|Default|SetMainMenuRef _returnvalue_2))
  (UserInterface|Viewport|AddtoViewport _output_get 0)
  (Variables|/Script/Engine.PlayerController|SetbShowMouseCursor _returnvalue true)
  (Input|SetInputModeGameandUI _returnvalue _output_get "DoNotLock" true false)
  (Default|ControllerHoverPlay (Variables|Default|GetMainMenuRef)))

(event Input|KeyboardEvents|Up
  (params (Key :type Key%20Structure :default "None"))
  (bind _mainmenuref (Variables|Default|GetMainMenuRef))
  (:Pressed
    (if (<= (Variables|Default|Getindex) 0)
      (Variables|Default|Setindex 0)
      (else
        (Math|Integer|DecrementInt (Variables|Default|Getindex)
          (:%20%20
            _))))
    (switch int (Variables|Default|Getindex)
      (:0
        (Default|ControllerHoverPlay _mainmenuref))
      (:1
        (Default|ControllerHoverQuit _mainmenuref)))))

(event Input|KeyboardEvents|Down
  (params (Key :type Key%20Structure :default "None"))
  (bind _mainmenuref (Variables|Default|GetMainMenuRef))
  (:Pressed
    (if (>= (Variables|Default|Getindex) (Variables|Default|GetnbMaxButtons))
      (Variables|Default|Setindex (Variables|Default|GetnbMaxButtons))
      (else
        (Math|Integer|IncrementInt (Variables|Default|Getindex)
          (:%20%20
            _))))
    (switch int (Variables|Default|Getindex)
      (:0
        (Default|ControllerHoverPlay _mainmenuref))
      (:1
        (Default|ControllerHoverQuit _mainmenuref)))))

(event Input|KeyboardEvents|Enter
  (params (Key :type Key%20Structure :default "None"))
  (bind _mainmenuref (Variables|Default|GetMainMenuRef))
  (:Pressed
    (switch int (Variables|Default|Getindex)
      (:0
        (Default|ControllerClickPlay _mainmenuref))
      (:1
        (Default|ControllerClickQuit _mainmenuref)))))

(event Input|GamepadEvents|GamepadDPadUp
  (params (Key :type Key%20Structure :default "None"))
  (bind _mainmenuref (Variables|Default|GetMainMenuRef))
  (:Pressed
    (if (<= (Variables|Default|Getindex) 0)
      (Variables|Default|Setindex 0)
      (else
        (Math|Integer|DecrementInt (Variables|Default|Getindex)
          (:%20%20
            _))))
    (switch int (Variables|Default|Getindex)
      (:0
        (Default|ControllerHoverPlay _mainmenuref))
      (:1
        (Default|ControllerHoverQuit _mainmenuref)))))

(event Input|GamepadEvents|GamepadDPadDown
  (params (Key :type Key%20Structure :default "None"))
  (bind _mainmenuref (Variables|Default|GetMainMenuRef))
  (:Pressed
    (if (>= (Variables|Default|Getindex) (Variables|Default|GetnbMaxButtons))
      (Variables|Default|Setindex (Variables|Default|GetnbMaxButtons))
      (else
        (Math|Integer|IncrementInt (Variables|Default|Getindex)
          (:%20%20
            _))))
    (switch int (Variables|Default|Getindex)
      (:0
        (Default|ControllerHoverPlay _mainmenuref))
      (:1
        (Default|ControllerHoverQuit _mainmenuref)))))

(event Input|GamepadEvents|GamepadFaceButtonBottom
  (params (Key :type Key%20Structure :default "None"))
  (bind _mainmenuref (Variables|Default|GetMainMenuRef))
  (:Pressed
    (switch int (Variables|Default|Getindex)
      (:0
        (Default|ControllerClickPlay _mainmenuref))
      (:1
        (Default|ControllerClickQuit _mainmenuref)))))

(fn ConstructionScript)