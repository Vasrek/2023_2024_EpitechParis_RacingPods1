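; BP_Bird is the bird pawn Blueprint, which here handles the HUD and an in-game pause menu.
; BeginPlay creates WBP_HUD and adds it to the viewport.
; The P key flip-flops between showing a new WBP_InGameMenuPause and removing it.
; The menu slows global time dilation rather than truly pausing, switches to Game and UI input and ignores move and look input, all restored on close.
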(event EventBeginPlay
  (bind _returnvalue (UserInterface|CreateWidget "/Game/Blueprints/Widgets/WBP_HUD.WBP_HUD_C"))
  (UserInterface|Viewport|AddtoViewport _returnvalue 0))

(event Input|KeyboardEvents|P
  (params (Key :type Key%20Structure :default "None"))
  (bind _returnvalue (Game|GetPlayerController 0))
  (bind _returnvalue_2 (Game|GetPlayerController 0))
  (:Pressed
    (Utilities|FlowControl|FlipFlop
      (:A
        (bind _returnvalue_3 (UserInterface|CreateWidget "/Game/Blueprints/Widgets/WBP_InGameMenuPause.WBP_InGameMenuPause_C"))
        (bind _output_get (Variables|Default|SetInGamePauseMenu _returnvalue_3))
        (UserInterface|Viewport|AddtoViewport _output_get 0)
        (Utilities|Time|SetGlobalTimeDilation 0.2)
        (Input|SetInputModeGameandUI _returnvalue _output_get "DoNotLock" true false)
        (Input|SetIgnoreMoveInput _returnvalue true)
        (Input|SetIgnoreLookInput _returnvalue true))
      (:B
        (Utilities|IsValid (Variables|Default|GetInGamePauseMenu)
          (:Is%20Valid
            (Widget|RemovefromParent (Variables|Default|GetInGamePauseMenu))
            (Utilities|Time|SetGlobalTimeDilation 1.0)
            (Variables|/Script/Engine.PlayerController|SetbShowMouseCursor _returnvalue_2 false)
            (Input|SetInputModeGameOnly _returnvalue_2 false)
            (Input|SetIgnoreMoveInput _returnvalue false)
            (Input|SetIgnoreLookInput _returnvalue false)))))))

(fn ConstructionScript)